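; FireWorksControl_BP launches a randomly colored firework at the player character's mesh location each time the left mouse button is pressed.
; It spawns the FireWorks_P particle emitter and creates a dynamic instance of M_FireworksTwo on it.
; The instance's Color parameter takes a random entry from ColorSelection, and the same instance is assigned to two of the emitter's material slots so they match.
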(event `Key|LeftMouseButton`
  (params (Key :type "Key Structure"))
  (:`Pressed`
    (bind _returnvalue (`GameplayStatics.SpawnEmitterAtLocation` "/Game/TS_Fireworks/Particles/FireWorks_P.FireWorks_P" (`SceneComponent.K2_GetComponentLocation` (`Character.Mesh` (`GameplayStatics.GetPlayerCharacter` 0)))))
    (bind _returnvalue_2 (`PrimitiveComponent.CreateDynamicMaterialInstance` _returnvalue 2 "/Game/TS_Fireworks/Materials/M_FireworksTwo.M_FireworksTwo" "None"))
    (`MaterialInstanceDynamic.SetVectorParameterValue` _returnvalue_2 "Color" (`|GetArrayItem` (`self.ColorSelection`) (`KismetMathLibrary.RandomIntegerInRange` 0 5)))
    (`PrimitiveComponent.SetMaterial` _returnvalue 3 _returnvalue_2)
    (`PrimitiveComponent.SetMaterial` _returnvalue 2 _returnvalue_2)))

(fn `UserConstructionScript`)